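; Actor component that shows damage screen effects through a camera-attached plane with a dynamic post-process material.
; On BeginPlay it creates the plane mesh, attaches it to the owner's camera and hides it.
; ShowDamageVFX takes a damage type, hiding the plane at full HP or showing it with a scale speed for low and critical HP.
; Instant damage runs a reusable looping timer that fades and scales the effect, then pauses and hides it.
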(event `self.ReceiveBeginPlay`
  (`self.Init`))

(fn `DecreasingOpacity`
  (if (> (`self.VFXOpacity`) 0.0)
    (`MaterialInstanceDynamic.SetScalarParameterValue` (`self.PostProcessDynMat`) (`self.OpacityName`) (`self.VFXOpacity`))
    (set `self.VFXOpacity` (- (`self.VFXOpacity`) 0.1))
    (`MaterialInstanceDynamic.SetScalarParameterValue` (`self.PostProcessDynMat`) (`self.DamageScaleUVName`) (`self.VFXDamageScale`))
    (set `self.VFXDamageScale` (+ (`self.VFXDamageScale`) 0.1))
    (else
      (`KismetSystemLibrary.K2_PauseTimerHandle` (`self.InstaDamageTimer`))
      (`self.Invalidate Post Process`)
      (`self.SetVFXVisibility` false))))

(fn `Init`
  (`|ExecutionSequence`
    (:`then_0`
      ;[1 1 1] Creating and attaching component
      (bind _returnvalue (`|AddComponentByClass` (`self.GetOwner`) "/Script/Engine.StaticMeshComponent" false (`KismetMathLibrary.MakeTransform` (75.0 0.0 0.0) (struct) (1.0 1.0 0.5))))
      (set `self.StaticMeshComponent` _returnvalue)
      (`SceneComponent.K2_AttachToComponent` (`self.StaticMeshComponent`) (`Actor.GetComponentByClass` (`self.GetOwner`) "/Script/Engine.CameraComponent") "None" "KeepRelative" "KeepRelative" "KeepRelative" true)
      ;[1 1 1] Creating and setting dynamic material
      (`StaticMeshComponent.SetStaticMesh` (`self.StaticMeshComponent`) "/Game/DamagePostProcess/SM_VFXPlane.SM_VFXPlane")
      (`PrimitiveComponent.SetCollisionEnabled` (`self.StaticMeshComponent`) "NoCollision")
      (bind _returnvalue_2 (`KismetMaterialLibrary.CreateDynamicMaterialInstance` "/Game/DamagePostProcess/M_PlanePostProcess.M_PlanePostProcess"))
      (set `self.PostProcessDynMat` _returnvalue_2)
      (`PrimitiveComponent.SetMaterial` (`self.StaticMeshComponent`) 0 (`self.PostProcessDynMat`)))
    (:`then_1`
      (`self.SetVFXVisibility` false))))

(fn `Invalidate Post Process`
  (set `self.VFXOpacity` 1.0)
  (set `self.VFXDamageScale` 1.0)
  (set `self.SpeedScaleVFX` 1.0)
  (`MaterialInstanceDynamic.SetScalarParameterValue` (`self.PostProcessDynMat`) (`self.OpacityName`) (`self.VFXOpacity`))
  (`MaterialInstanceDynamic.SetScalarParameterValue` (`self.PostProcessDynMat`) (`self.DamageScaleUVName`) (`self.VFXDamageScale`))
  (`MaterialInstanceDynamic.SetScalarParameterValue` (`self.PostProcessDynMat`) (`self.SpeedScaleVFXName`) (`self.SpeedScaleVFX`)))

(fn `RunInstaDamageVFX`
  (if (not (`KismetSystemLibrary.K2_TimerExistsHandle` (`self.InstaDamageTimer`)))
    (bind _returnvalue (`KismetSystemLibrary.K2_SetTimer` null "DecreasingOpacity" 0.025 true))
    (set `self.InstaDamageTimer` _returnvalue)
    (else
      (if (`KismetSystemLibrary.K2_IsTimerActiveHandle` (`self.InstaDamageTimer`))
        (`self.Invalidate Post Process`))
      (`KismetSystemLibrary.K2_UnPauseTimerHandle` (`self.InstaDamageTimer`)))))

(fn `SetVFXVisibility`
  (params (IsVisibled :type Boolean))
  (`SceneComponent.SetVisibility` (`self.StaticMeshComponent`) IsVisibled false))

(fn `ShowDamageVFX`
  (params (InDamageType :type "/Game/DamagePostProcess/E_VFXDamageType Enum" :default "NewEnumerator2"))
  ;[1 1 1] Set Scale Speed
  (set `self.SpeedScaleVFX` (select `/Game/DamagePostProcess/E_VFXDamageType` (`local.InDamageType`) :`NewEnumerator2` 0.0 :`NewEnumerator1` (`self.LowHPDamageScaleSpeed`) :`NewEnumerator3` (`self.CriticalHPDamageScaleSpeed`)))
  (`MaterialInstanceDynamic.SetScalarParameterValue` (`self.PostProcessDynMat`) (`self.SpeedScaleVFXName`) (`self.SpeedScaleVFX`))
  (switch `/Game/DamagePostProcess/E_VFXDamageType` (`local.InDamageType`)
    (:`NewEnumerator2`
      (`self.SetVFXVisibility` false))
    (:`NewEnumerator0`
      (`self.RunInstaDamageVFX`)
      (`self.SetVFXVisibility` true :!label _label))
    (:`NewEnumerator1`
      (goto _label))
    (:`NewEnumerator3`
      (goto _label))))